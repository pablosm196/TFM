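; Test AI controller that runs the BT_U1_2 behavior tree on possess and feeds perception results into its Blackboard.
; Sensing an actor tagged "Objective" cancels the forget timer and sets HasLineOfSight and Enemy.
; Any other perception update starts a LineOfSightTimer-length timer that clears both keys on expiry, delaying target loss.
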(event OnTargetPerceptionUpdated(AIPerception)
  (params (Actor :type Actor%20Object%20Reference) (Stimulus :type AI%20Stimulus%20Structure))
  (bind _blackboard (Variables|Default|GetBlackboard))
  (if (and (Actor|ActorHasTag Actor "Objective") (.bSuccessfullySensed (Utilities|Struct|BreakAIStimulus Stimulus)))
    (Utilities|Time|ClearandInvalidateTimerbyHandle (Variables|Default|GetObjectiveTimer))
    (AI|Components|Blackboard|SetValueasBool _blackboard (Variables|Default|GetHasLineOfSight?) true)
    (AI|Components|Blackboard|SetValueasObject _blackboard (Variables|Default|GetEnemy) Actor)
    (else
      (bind _returnvalue (Utilities|Time|SetTimerbyEvent (delegate Custom|StartObjectiveTimer) (Variables|Default|GetLineOfSightTimer)))
      (Variables|Default|SetObjectiveTimer _returnvalue))))

(event Custom|StartObjectiveTimer
  (bind _blackboard (Variables|Default|GetBlackboard))
  (AI|Components|Blackboard|SetValueasBool _blackboard (Variables|Default|GetHasLineOfSight?) false)
  (AI|Components|Blackboard|SetValueasObject _blackboard (Variables|Default|GetEnemy) 0))

(event EventPossess
  (params (PossessedPawn :type Pawn%20Object%20Reference))
  (AI|RunBehaviorTree "/Game/TFM/BTs_Pruebas/BT_U1_2.BT_U1_2"))

(fn ConstructionScript)